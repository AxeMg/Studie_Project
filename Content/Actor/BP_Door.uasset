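; BP_Door is an interactable swinging door that can start locked or shut and lock itself behind a trigger.
; Interact alternates opening and closing through a FlipFlop timeline that lerps mesh yaw, or plays a locked-door rotation when locked.
; If CanBeLocked is set, overlapping Box_Locking sets IsLocked once and animates the door to zero yaw.
; Box_Prompt overlaps show and hide the prompt widget.
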(event `/Game/FirstPerson/Blueprints/BPI_Interact.Interact`
  (params (Player :type "/Game/FirstPerson/Blueprints/BP_FirstPersonCharacter Object Reference"))
  (if (or (`self.IsLocked`) (`self.Locked`))
    ;[1 1 1] Porte bloquée
    (bind (_direction _doorlocked) (`Timeline|DoorLocked` :!via `PlayFromStart`)
      (:`Update`
        (`SceneComponent.K2_SetRelativeRotation` (`self.SM_Door_StaticMeshComponent0`) (`KismetMathLibrary.MakeRotator` 0.0 0.0 _doorlocked) false false)))
    (else
      ;[1 1 1] Ouverture porte
      (`/Engine/EditorBlueprintResources/StandardMacros.FlipFlop`
        (:`A`
          (bind (_direction_2 _door) (`Timeline|DoorAnim` :!label _label)
            (:`Update`
              (`SceneComponent.K2_SetRelativeRotation` (`self.SM_Door_StaticMeshComponent0`) (`KismetMathLibrary.MakeRotator` 0.0 0.0 (`KismetMathLibrary.Lerp` (`self.DoorAngle`) (`self.DoorOpenAngle`) _door)) false false))))
        (:`B`
          (goto _label :!via `Reverse`))))))

(event `self.Box_Locking.OnComponentBeginOverlap`
  (params (OverlappedComponent :type "PrimitiveComponent Object Reference") (OtherActor :type "Actor Object Reference") (OtherComp :type "PrimitiveComponent Object Reference") (OtherBodyIndex :type Integer) (bFromSweep :type Boolean) (SweepResult :type "HitResult Structure (by ref)"))
  ;[1 1 1] Fermeture porte
  (if (`self.CanBeLocked`)
    (if (not (`self.IsLocked`))
      (set `self.IsLocked` true)
      (bind (_direction _doorclosing) (`Timeline|DoorClosing`)
        (:`Update`
          (bind _returnvalue (`KismetMathLibrary.Lerp` (`self.DoorOpenAngle`) 0.0 _doorclosing))
          (set `self.DoorAngle` _returnvalue)
          (`SceneComponent.K2_SetRelativeRotation` (`self.SM_Door_StaticMeshComponent0`) (`KismetMathLibrary.MakeRotator` 0.0 0.0 _returnvalue) false false))))))

(event `self.Box_Prompt.OnComponentBeginOverlap`
  (params (OverlappedComponent :type "PrimitiveComponent Object Reference") (OtherActor :type "Actor Object Reference") (OtherComp :type "PrimitiveComponent Object Reference") (OtherBodyIndex :type Integer) (bFromSweep :type Boolean) (SweepResult :type "HitResult Structure (by ref)"))
  (`SceneComponent.SetHiddenInGame` (`self.Widget`) false false))

(event `self.Box_Prompt.OnComponentEndOverlap`
  (params (OverlappedComponent :type "PrimitiveComponent Object Reference") (OtherActor :type "Actor Object Reference") (OtherComp :type "PrimitiveComponent Object Reference") (OtherBodyIndex :type Integer))
  (`SceneComponent.SetHiddenInGame` (`self.Widget`) true false))

(fn `UserConstructionScript`)